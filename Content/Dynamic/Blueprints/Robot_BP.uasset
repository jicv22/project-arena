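; Robot character Blueprint with player-driven camera, control-yaw-relative movement, jumping and sprinting, plus a jump event intended for AI.
; AIJump launches the character toward a target along a suggested projectile arc scaled by a booster, then a short timer ends the jump.
; Sprint toggles walk and sprint speed and acceleration, while movement and jump inputs update state flags.
; Holding Attack only slows global time as a placeholder action.
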(event `self.ReceiveBeginPlay`
  (bind _charactermovement (`self.CharacterMovement`))
  ;[1 1 1] BeginPlay
  (set `CharacterMovementComponent.MaxAcceleration` (`self.MaxWalkAcceleration`) _charactermovement)
  (set `CharacterMovementComponent.MaxWalkSpeed` (`self.MaxWalkSpeed`) _charactermovement))

(event `InputAxis|CameraTurn`
  (params (AxisValue :type "Float (single-precision)"))
  ;[1 1 1] Camera Movement
  (`self.AddControllerYawInput` AxisValue))

(event `InputAxis|CameraUp`
  (params (AxisValue :type "Float (single-precision)"))
  ;[1 1 1] Camera Movement
  (`self.AddControllerPitchInput` AxisValue))

(event `InputAxis|MoveForward`
  (params (AxisValue :type "Float (single-precision)"))
  (bind (_returnvalue_roll _returnvalue_pitch _returnvalue_yaw) (`KismetMathLibrary.BreakRotator` (`self.GetControlRotation`)))
  ;[1 1 1] Character Movement
  (`self.AddMovementInput` (`KismetMathLibrary.GetForwardVector` (`KismetMathLibrary.MakeRotator` 0.0 0.0 _returnvalue_yaw)) AxisValue)
  (if (or (!= AxisValue 0.0) (!= (stale `InputAxis|MoveRight` AxisValue) 0.0)) :!label _label
    (set `self.isMovingWithKeyboard` true)
    (else
      (set `self.isMovingWithKeyboard` false))))

(event `InputAxis|MoveRight`
  (params (AxisValue :type "Float (single-precision)"))
  (bind (_returnvalue_roll _returnvalue_pitch _returnvalue_yaw) (`KismetMathLibrary.BreakRotator` (`self.GetControlRotation`)))
  ;[1 1 1] Character Movement
  (`self.AddMovementInput` (`KismetMathLibrary.GetRightVector` (`KismetMathLibrary.MakeRotator` 0.0 0.0 _returnvalue_yaw)) AxisValue)
  (goto _label))

(event `AIJump`
  (params (TargetLocatione :type "Vector Structure") (JumpBooster :type "Float (double-precision)"))
  ;[1 1 1] Jump With AI
  (set `self.IsJumping` true)
  (bind _outlaunchvelocity (`GameplayStatics.SuggestProjectileVelocity_CustomArc` (`self.K2_GetActorLocation`) TargetLocatione))
  (`self.LaunchCharacter` (* _outlaunchvelocity JumpBooster) true)
  (`KismetSystemLibrary.K2_SetTimerDelegate` (delegate `AIStopJump`) 0.1))

(event `AIStopJump`
  ;[1 1 1] Jump With AI
  (set `self.IsJumping` false)
  (`self.StopJumping`))

(event `InputAction|Jump`
  (params (Key :type "Key Structure"))
  ;[1 1 1] Jump for Player
  (:`Pressed`
    (set `self.IsJumping` true)
    (`self.Jump`)
    (`KismetSystemLibrary.Delay` 0.01)
    (set `self.IsJumping` false))
  (:`Released`
    (set `self.IsJumping` false)
    (`self.StopJumping`)))

(event `InputAction|Sprint`
  (params (Key :type "Key Structure"))
  (bind _charactermovement (`self.CharacterMovement`))
  ;[1 1 1] Character Sprint
  (:`Pressed`
    (bind _isa (`/Engine/EditorBlueprintResources/StandardMacros.FlipFlop`)
      (:`A`
        (set `self.isSprinting` _isa)
        (set `CharacterMovementComponent.MaxAcceleration` (`self.MaxSprintAcceleration`) _charactermovement)
        (set `CharacterMovementComponent.MaxWalkSpeed` (`self.MaxSprintSpeed`) _charactermovement))
      (:`B`
        (set `self.isSprinting` _isa)
        (set `CharacterMovementComponent.MaxAcceleration` (`self.MaxWalkAcceleration`) _charactermovement)
        (set `CharacterMovementComponent.MaxWalkSpeed` (`self.MaxWalkSpeed`) _charactermovement)))))

(event `InputAction|Attack`
  (params (Key :type "Key Structure"))
  ;[1 1 1] Character Action (Look for something to do with this)
  (:`Pressed`
    (`GameplayStatics.SetGlobalTimeDilation` 0.15))
  (:`Released`
    (`GameplayStatics.SetGlobalTimeDilation` 1.0)))

(fn `UserConstructionScript`)