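; AI controller for enemy robot characters that runs their behavior tree on possession.
; AI perception writes sensed actors tagged both Robot and Player to the blackboard as the visible enemy.
; Losing perception of an actor clears the sight flag, saves that actor's location as the target, and starts a timer that forgets the enemy after a configurable delay.
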(event `self.ReceivePossess`
  (params (PossessedPawn :type "Pawn Object Reference"))
  (bind _ascharacter_bp (cast `/Game/Dynamic/Blueprints/Character_BP` PossessedPawn))
  (set `self.PossessedRobot` _ascharacter_bp)
  (`self.RunBehaviorTree` "/Game/Dynamic/Blueprints/AI/Robot_Enemy_BT.Robot_Enemy_BT"))

(event `ClearEnemyOnMemory`
  (`BlackboardComponent.SetValueAsObject` (`self.Blackboard`) (`self.EnemyActorKey`) null))

(event `self.AIPerception.OnTargetPerceptionUpdated`
  (params (Actor :type "Actor Object Reference") (Stimulus :type "AIStimulus Structure"))
  (bind _blackboard (`self.Blackboard`))
  (bind _blackboard_2 (`self.Blackboard`))
  (if (`.bSuccessfullySensed` (break `AIStimulus` Stimulus))
    (if (`self.ActorHasTag` Actor "Robot")
      (if (`self.ActorHasTag` Actor "Player")
        (`BlackboardComponent.SetValueAsObject` _blackboard_2 (`self.EnemyActorKey`) Actor)
        (`BlackboardComponent.SetValueAsBool` _blackboard_2 (`self.IsEnemyOnSightKey`) true)))
    (else
      (`KismetSystemLibrary.K2_SetTimerDelegate` (delegate `ClearEnemyOnMemory`) (`self.TimeToForgotEnemy`))
      (`BlackboardComponent.SetValueAsBool` _blackboard (`self.IsEnemyOnSightKey`) false)
      (`BlackboardComponent.SetValueAsVector` _blackboard (`self.TargetLocationKey`) (`self.K2_GetActorLocation` Actor)))))

(fn `UserConstructionScript`)