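; TripLeg_BP is a Blueprint subclass that supplies movement and camera tuning for what appears to be a third-person character.
; On BeginPlay it sets walk and sprint speed and acceleration, plus spring arm length and socket offset for normal and aiming views.
; These values are assigned before the parent BeginPlay runs; using them is left to the parent class.
; The construction script only calls its parent.
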(event `self.ReceiveBeginPlay`
  (set `self.MaxWalkAcceleration` 600.0)
  (set `self.MaxSprintAcceleration` 1200.0)
  (set `self.MaxWalkSpeed` 300.0)
  (set `self.MaxSprintSpeed` 600.0)
  (set `self.TargetArmLength` 300.0)
  (set `self.AimingTargetArmLength` 150.0)
  (set `self.SpringArmSocketOffset` (0.0 0.0 0.0))
  (set `self.AimingSpringArmSocketOffset` (0.0 25.0 25.0))
  (`parent.ReceiveBeginPlay`))

(fn `UserConstructionScript`
  (`parent.UserConstructionScript`))